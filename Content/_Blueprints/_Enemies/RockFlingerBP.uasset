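; RockFlingerBP is an enemy that carries a body of rocks and flings them at the player.
; On initialization it spawns NumOrbitals Rocks actors at its location into the Body array and caches the player pawn as MainPlayer.
; A looping timer fires every few seconds, homing a random rock on the player's current location.
; It then removes a separately randomized entry from Body, which may differ from the launched rock, and never refills it.
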(event Custom|Fire
  (bind _body (Variables|Default|GetBody))
  (bind _body_2 (Variables|Default|GetBody))
  (bind _returnvalue (Utilities|Array|Length _body_2))
  (bind _returnvalue_2 (- _returnvalue 1))
  (bind _returnvalue_3 (Math|Random|RandomIntegerinRange 0 _returnvalue_2))
  (bind _output (Utilities|Array|Get(acopy) _body _returnvalue_3))
  (Default|Home _output (Transformation|GetActorLocation (Variables|Default|GetPlayerREF)))
  (Utilities|Array|RemoveItem _body _output))

(event EventInitialize
  (bind _returnvalue (Transformation|GetActorLocation))
  (|CallParentFunction)
  (Utilities|FlowControl|Sequence
    (:then_0
      (Utilities|FlowControl|ForLoopwithBreak 0 (- (Variables|Default|GetNumOrbitals) 1)
        (:LoopBody
          (bind _returnvalue_2 (Game|SpawnActorfromClass "/Game/_Blueprints/_Enemies/Rocks.Rocks_C" (Math|Transform|MakeTransform _returnvalue "0, 0, 0" "1.000000,1.000000,1.000000") "Undefined" 0 _returnvalue 0))
          (Utilities|Array|Add (Variables|Default|GetBody) _returnvalue_2))))
    (:then_1
      (Utilities|Time|SetTimerbyEvent (delegate Custom|Fire) 3.0 true)
      (bind _asmain_player (Utilities|Casting|CastToMainPlayer (Game|Player|GetPlayerPawn 0)))
      (Variables|Default|SetPlayerREF _asmain_player))))

(fn ConstructionScript
  (|CallParentFunction))