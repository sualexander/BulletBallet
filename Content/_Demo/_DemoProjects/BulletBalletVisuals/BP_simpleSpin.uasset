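; BP_simpleSpin is a demo actor in the BulletBalletVisuals project that spins a set of meshes about their Z axis.
; The construction script gathers its mesh components into the AllMeshes array.
; On BeginPlay the Spin timeline starts, and each update sets every mesh's relative rotation from the timeline's 1TOPI track as the angle.
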(event EventBeginPlay
  (bind _1topi (Timeline|Spin Play)
    (:Update
      (for _array_element (Variables|Default|GetAllMeshes)
        (Transformation|SetRelativeRotation _array_element (Math|Vector|RotatorfromAxisandAngle "0, 0,1.000000" _1topi) false false)))))

(event Collision|EventActorBeginOverlap
  (params (OtherActor :type Actor%20Object%20Reference)))

(event EventTick
  (params (DeltaSeconds :type Float%20%28single-precision%29)))

(fn ConstructionScript
  (Variables|Default|SetAllMeshes (Utilities|Array|MakeArray (Variables|Default|Gettestmesh) (Variables|Default|Gettestmesh1) (Variables|Default|Gettestmesh2) (Variables|Default|Gettestmesh4) (Variables|Default|Gettestmesh5) (Variables|Default|Gettestmesh7) (Variables|Default|Gettestmesh8) 0)))