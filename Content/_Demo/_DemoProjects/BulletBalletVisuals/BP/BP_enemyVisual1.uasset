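; Enemy visual actor for the Bullet Ballet visuals demo, with a spinning static mesh and a flickering point light.
; BeginPlay starts two looping 0.1-second timers in place of Tick.
; SpinMesh sets the mesh's yaw from game time scaled by SpinSpeed, while LightFlicker drives intensity with a time-based sine floored at BaseLightIntensity.
; The construction script creates a dynamic material instance and sets the initial light intensity.
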(event EventBeginPlay
  (Utilities|Time|SetTimerbyFunctionName 0 "SpinMesh" 0.1 true)
  (Utilities|Time|SetTimerbyFunctionName 0 "LightFlicker" 0.1 true))

(event Collision|EventActorBeginOverlap
  (params (OtherActor :type Actor%20Object%20Reference)))

(event EventTick
  (params (DeltaSeconds :type Float%20%28single-precision%29)))

(fn ConstructionScript
  (bind _returnvalue (Rendering|Material|CreateDynamicMaterialInstance (Variables|Default|Getstaticmesh) 0 0 "None" :!class /Script/Engine.PrimitiveComponent))
  (Variables|Default|SetMatInst _returnvalue)
  (Rendering|Components|Light|SetIntensity (Variables|Default|GetPointLight) (Variables|Default|GetLightIntensity)))

(fn SpinMesh
  (Transformation|SetRelativeRotation (Variables|Default|Getstaticmesh) (Math|Vector|RotatorfromAxisandAngle "0, 0,1.000000" (/ (Utilities|Time|GetGameTimeinSeconds) (/ 1.0 (Variables|Default|GetSpinSpeed)))) false false))

(fn LightFlicker
  (Rendering|Components|Light|SetIntensity (Variables|Default|GetPointLight) (Math|Float|Max(Float) (* (Math|Trig|Sin(Degrees) (/ (Utilities|Time|GetGameTimeinSeconds) (/ 1.0 (Variables|Default|GetFlickerSpeed)))) (Variables|Default|GetLightIntensity)) (Variables|Default|GetBaseLightIntensity))))