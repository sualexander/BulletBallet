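; BP_Enemy is a collision-event demo enemy that drives a configurable Niagara effect reporting back to a player reference.
; The Construction Script assigns the Niagara system, tints it through DamageColor and passes PlayerRef as the BPCallback object so the player can receive particle events.
; On BeginPlay it adds its Niagara asset to the player's detect list.
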(event EventBeginPlay
  (Default|AddtoDetectList (Variables|Default|GetPlayerRef) (AssetData|GetAsset (Variables|Default|GetNiagara))))

(event Collision|EventActorBeginOverlap
  (params (OtherActor :type Actor%20Object%20Reference)))

(event EventTick
  (params (DeltaSeconds :type Float%20%28single-precision%29)))

(fn ConstructionScript
  (bind _niagara (Variables|Default|GetNiagara))
  ;[1 1 1] set the type of niagara system used
  (Class|NiagaraComponent|SetAsset (Variables|Default|GetNiagara) (Variables|Default|GetNiagaraType) true)
  ;[1 1 1] set color cuz nice
  (Niagara|SetNiagaraVariable(LinearColor) _niagara "DamageColor" (Variables|Default|GetColor))
  ;[1 1 1] set up reference such that it can receive blueprint events
  (Class|NiagaraComponent|SetVariableObject _niagara "BPCallback" (Variables|Default|GetPlayerRef)))