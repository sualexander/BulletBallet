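; BP_CollisionReceiver is a demo actor that counts collision events delivered as particle data and shows the running total on a text render.
; Each ParticleData event adds the length of its data array to CollisionCounter and updates the text.
; The D and G keys nudge the root along Y in fixed, unswept steps.
; AddToDetectList appends projectiles to DetectList, which nothing here reads.
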(event EventBeginPlay)

(event Collision|EventActorBeginOverlap
  (params (OtherActor :type Actor%20Object%20Reference)))

(event EventTick
  (params (DeltaSeconds :type Float%20%28single-precision%29)))

(event EventParticleData
  (params (Data :type Array%20of%20Basic%20Particle%20Data%20Structures) (NiagaraSystem :type Niagara%20System%20Object%20Reference) (SimulationPositionOffset :type Vector%20%28by%20ref%29 :default "0, 0, 0"))
  (bind _output_get (Variables|Default|SetCollisionCounter (+ (Variables|Default|GetCollisionCounter) (Utilities|Array|Length Data))))
  (Rendering|Components|TextRender|SetText (Variables|Default|GetTextRender) (Utilities|Text|ToText(Integer) _output_get)))

(event Input|KeyboardEvents|D
  (params (Key :type Key%20Structure :default "None"))
  ;[1 1 1] extremely basic moving left and right
  (:Pressed
    (Transformation|AddWorldOffset (Variables|Default|GetDefaultSceneRoot) "0,-15.000000, 0" false false)))

(event Input|KeyboardEvents|G
  (params (Key :type Key%20Structure :default "None"))
  ;[1 1 1] extremely basic moving left and right
  (:Pressed
    (Transformation|AddWorldOffset (Variables|Default|GetDefaultSceneRoot) "0,15.000000, 0" false false)))

(fn ConstructionScript)

(fn AddtoDetectList
  (params (NewProjectile :type Niagara%20System%20Object%20Reference))
  (Utilities|Array|Add (Variables|Default|GetDetectList) NewProjectile))